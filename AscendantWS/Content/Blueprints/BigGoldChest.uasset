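; BigGoldChest is a loot chest actor that drops one item when an interaction is detected, then destroys itself.
; InteractDetect calls GenerateItems, which makes a random percentage roll to pick the item class, favoring RareItem (about 70%) over UncommonItem.
; The chosen item spawns at a fixed height above the chest's location before the chest is removed.
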(event EventInteractDetect
  (params (Target :type Object%20Object%20Reference))
  (CallFunction|GenerateItems)
  (Actor|DestroyActor))

(fn ConstructionScript)

(fn GenerateItems
  (if (>= (Math|Random|RandomFloatinRange 0.0 1e+02) 7e+01)
    (Game|SpawnActorfromClass "/Game/Blueprints/UncommonItem.UncommonItem_C" (Math|Conversions|ToTransform(Vector) (+ (Transformation|GetActorLocation) "0.000000, 0,150.000000")) "Undefined" 0 0)
    (else
      (Game|SpawnActorfromClass "/Game/Blueprints/RareItem.RareItem_C" (Math|Conversions|ToTransform(Vector) (+ (Transformation|GetActorLocation) "0, 0,150.000000")) "Undefined" 0 0))))