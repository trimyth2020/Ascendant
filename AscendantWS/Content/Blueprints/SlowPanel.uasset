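; SlowPanel is a single-use trap that temporarily slows a PlayerCharB that steps into its trigger.
; On overlap it scales the character's MaxWalkSpeed by SlowFraction, disables the trigger's collision and hides the Cube mesh.
; After a SlowTime delay it sets walk speed to a hardcoded default, rather than the saved prior value, and destroys itself.
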(event OnComponentBeginOverlap(SlowTrapTrigger)
  (params (OverlappedComponent :type Primitive%20Component%20Object%20Reference) (OtherActor :type Actor%20Object%20Reference) (OtherComp :type Primitive%20Component%20Object%20Reference) (OtherBodyIndex :type Integer) (bFromSweep :type Boolean) (SweepResult :type Hit%20Result%20Structure%20%28by%20ref%29))
  (bind _asplayer_char_b (Utilities|Casting|CastToPlayerCharB OtherActor))
  (Variables|/Script/Engine.CharacterMovementComponent|SetMaxWalkSpeed (Variables|/Script/Engine.Character|GetCharacterMovement _asplayer_char_b) (* (Variables|/Script/Engine.CharacterMovementComponent|GetMaxWalkSpeed (Variables|/Script/Engine.Character|GetCharacterMovement _asplayer_char_b)) (Variables|Default|GetSlowFraction)))
  (Collision|SetCollisionEnabled (Variables|Default|GetSlowTrapTrigger) "NoCollision")
  (Rendering|SetVisibility (Variables|Default|GetCube) false false)
  (Utilities|FlowControl|Delay (Variables|Default|GetSlowTime))
  (Variables|/Script/Engine.CharacterMovementComponent|SetMaxWalkSpeed (Variables|/Script/Engine.Character|GetCharacterMovement _asplayer_char_b) 6e+02)
  (Actor|DestroyActor))

(fn ConstructionScript)