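; One-shot item spawner that drops random common loot at its location on BeginPlay, then destroys itself.
; A weighted roll picks one branch: gold, a key, a stat rune with a pile of gold, or an elemental rune chosen by a second even roll.
; Keys and stat runes get a common marker particle and elemental runes an uncommon one.
; The SpawnGold loop's SpawnActor has no class set.
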(event EventBeginPlay
  (bind _output_get (Variables|Default|SetContentsChance (Math|Random|RandomFloatinRange 0.0 1e+02)))
  (Utilities|FlowControl|Sequence
    (:then_0
      (if (<= _output_get 35.0)
        (CallFunction|SpawnGold)
        (Actor|DestroyActor :!label _label)))
    (:then_1
      (if (and (> _output_get 35.0) (<= _output_get 6e+01))
        (CallFunction|SpawnKey)
        (goto _label)))
    (:then_2
      (if (and (> _output_get 6e+01) (<= _output_get 8e+01))
        (CallFunction|SpawnStat)
        (goto _label)))
    (:then_3
      (if (> _output_get 8e+01)
        (CallFunction|SpawnRune)
        (goto _label)))))

(fn ConstructionScript)

(fn SpawnRune
  (bind _defaultsceneroot (Variables|Default|GetDefaultSceneRoot))
  (bind _returnvalue (Transformation|GetWorldTransform _defaultsceneroot))
  (bind _returnvalue_2 (Transformation|GetWorldTransform _defaultsceneroot))
  (bind _returnvalue_3 (Transformation|GetWorldTransform _defaultsceneroot))
  (bind _returnvalue_4 (Transformation|GetWorldTransform _defaultsceneroot))
  (bind _output_get (Variables|Default|SetRuneChance (Math|Random|RandomFloatinRange 0.0 1e+02)))
  (Utilities|FlowControl|Sequence
    (:then_0
      (if (<= _output_get 25.0)
        (bind _returnvalue_5 (Game|SpawnActorfromClass :Class "/Game/Blueprints/Items/FireRuneItem.FireRuneItem_C" :SpawnTransform (Math|Transform|MakeTransform (.location _returnvalue) (.rotation _returnvalue) "1,1,1") :CollisionHandlingOverride "Undefined" :Instigator 0))
        (Effects|SpawnEmitterAttached "/Game/Particles/P_UncommonMarker.P_UncommonMarker" (Variables|/Game/Blueprints/Items/FireRuneItem.FireRuneItem_C|GetEmmit _returnvalue_5) "None")))
    (:then_1
      (if (and (> _output_get 25.0) (<= _output_get 5e+01))
        (bind _returnvalue_6 (Game|SpawnActorfromClass :Class "/Game/Blueprints/Items/WaterRuneItem.WaterRuneItem_C" :SpawnTransform (Math|Transform|MakeTransform (.location _returnvalue_2) (.rotation _returnvalue_2) "1,1,1") :CollisionHandlingOverride "Undefined" :Instigator 0))
        (Effects|SpawnEmitterAttached "/Game/Particles/P_UncommonMarker.P_UncommonMarker" (Variables|/Game/Blueprints/Items/WaterRuneItem.WaterRuneItem_C|GetEmmit _returnvalue_6) "None")))
    (:then_2
      (if (and (> _output_get 5e+01) (<= _output_get 75.0))
        (bind _returnvalue_7 (Game|SpawnActorfromClass :Class "/Game/Blueprints/Items/LightningRuneItem.LightningRuneItem_C" :SpawnTransform (Math|Transform|MakeTransform (.location _returnvalue_3) (.rotation _returnvalue_3) "1,1,1") :CollisionHandlingOverride "Undefined" :Instigator 0))
        (Effects|SpawnEmitterAttached "/Game/Particles/P_UncommonMarker.P_UncommonMarker" (Variables|/Game/Blueprints/Items/LightningRuneItem.LightningRuneItem_C|GetEmmit _returnvalue_7) "None")))
    (:then_3
      (if (> _output_get 75.0)
        (bind _returnvalue_8 (Game|SpawnActorfromClass :Class "/Game/Blueprints/Items/EarthRuneItem.EarthRuneItem_C" :SpawnTransform (Math|Transform|MakeTransform (.location _returnvalue_4) (.rotation _returnvalue_4) "1,1,1") :CollisionHandlingOverride "Undefined" :Instigator 0))
        (Effects|SpawnEmitterAttached "/Game/Particles/P_UncommonMarker.P_UncommonMarker" (Variables|/Game/Blueprints/Items/EarthRuneItem.EarthRuneItem_C|GetEmmit _returnvalue_8) "None")))))

(fn SpawnKey
  (bind _returnvalue (Transformation|GetActorTransform))
  (bind _returnvalue_2 (Game|SpawnActorfromClass "/Game/Blueprints/Items/Key.Key_C" (Math|Transform|MakeTransform (.location _returnvalue) (.rotation _returnvalue) "1,1,1") "Undefined" 0 0))
  (Effects|SpawnEmitterAttached "/Game/Particles/P_CommonMarker.P_CommonMarker" (Variables|/Game/Blueprints/Items/Key.Key_C|GetEmmit _returnvalue_2) "None"))

(fn SpawnGold
  (bind _returnvalue (Transformation|GetActorTransform))
  (for _index (range 0 20)
    (Game|SpawnActorfromClass "/Game/Blueprints/Gold.Gold_C" (Math|Transform|MakeTransform (.location _returnvalue) (.rotation _returnvalue) "1,1,1") "Undefined" 0 0)))

(fn SpawnStat
  (bind _defaultsceneroot (Variables|Default|GetDefaultSceneRoot))
  (bind _returnvalue (Transformation|GetWorldTransform _defaultsceneroot))
  (for _index (range 0 20)
    (Game|SpawnActorfromClass "/Game/Blueprints/Gold.Gold_C" (Math|Transform|MakeTransform (.location _returnvalue) (.rotation _returnvalue) "1,1,1") "Undefined" 0 0))
  (bind _returnvalue_2 (Game|SpawnActorfromClass :Class "/Game/Blueprints/Items/StatRuneItem.StatRuneItem_C" :SpawnTransform (Math|Transform|MakeTransform (.location _returnvalue) (.rotation _returnvalue) "1,1,1") :CollisionHandlingOverride "Undefined" :Instigator 0))
  (Effects|SpawnEmitterAttached "/Game/Particles/P_CommonMarker.P_CommonMarker" (Variables|/Game/Blueprints/Items/StatRuneItem.StatRuneItem_C|GetEmmit _returnvalue_2) "None"))