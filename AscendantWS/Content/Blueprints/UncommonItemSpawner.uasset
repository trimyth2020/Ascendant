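; Uncommon-tier loot spawner that drops a random reward at its own transform on BeginPlay.
; An even roll picks either SpawnGoldStat (a gold pile plus a StatRuneItem with a common marker, identical in all three branches) or SpawnWeapon (one of four weapons with an uncommon marker).
; SpawnRune and SpawnActive hold similar random tables for elemental runes and active items but are never called here, and SpawnPassive is empty.
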(event EventBeginPlay
  (if (> (Math|Random|RandomFloatinRange 0.0 1e+02) 5e+01)
    (CallFunction|SpawnGoldStat)
    (else
      (CallFunction|SpawnWeapon))))

(fn ConstructionScript)

(fn SpawnRune
  (bind _defaultsceneroot (Variables|Default|GetDefaultSceneRoot))
  (bind _returnvalue (Transformation|GetWorldTransform _defaultsceneroot))
  (bind _returnvalue_2 (Transformation|GetWorldTransform _defaultsceneroot))
  (bind _returnvalue_3 (Transformation|GetWorldTransform _defaultsceneroot))
  (bind _returnvalue_4 (Transformation|GetWorldTransform _defaultsceneroot))
  (bind _output_get (Variables|Default|SetRuneChance (Math|Random|RandomFloatinRange 0.0 1e+02)))
  (Utilities|FlowControl|Sequence
    (:then_0
      (if (<= _output_get 25.0)
        (bind _returnvalue_5 (Game|SpawnActorfromClass :Class "/Game/Blueprints/Items/FireRuneItem.FireRuneItem_C" :SpawnTransform (Math|Transform|MakeTransform (.location _returnvalue) (.rotation _returnvalue) "1,1,1") :CollisionHandlingOverride "Undefined" :Instigator 0))
        (Effects|SpawnEmitterAttached "/Game/Particles/P_UncommonMarker.P_UncommonMarker" (Variables|/Game/Blueprints/Items/FireRuneItem.FireRuneItem_C|GetEmmit _returnvalue_5) "None")))
    (:then_1
      (if (and (> _output_get 25.0) (<= _output_get 5e+01))
        (bind _returnvalue_6 (Game|SpawnActorfromClass :Class "/Game/Blueprints/Items/WaterRuneItem.WaterRuneItem_C" :SpawnTransform (Math|Transform|MakeTransform (.location _returnvalue_2) (.rotation _returnvalue_2) "1,1,1") :CollisionHandlingOverride "Undefined" :Instigator 0))
        (Effects|SpawnEmitterAttached "/Game/Particles/P_UncommonMarker.P_UncommonMarker" (Variables|/Game/Blueprints/Items/WaterRuneItem.WaterRuneItem_C|GetEmmit _returnvalue_6) "None")))
    (:then_2
      (if (and (> _output_get 5e+01) (<= _output_get 75.0))
        (bind _returnvalue_7 (Game|SpawnActorfromClass :Class "/Game/Blueprints/Items/LightningRuneItem.LightningRuneItem_C" :SpawnTransform (Math|Transform|MakeTransform (.location _returnvalue_3) (.rotation _returnvalue_3) "1,1,1") :CollisionHandlingOverride "Undefined" :Instigator 0))
        (Effects|SpawnEmitterAttached "/Game/Particles/P_UncommonMarker.P_UncommonMarker" (Variables|/Game/Blueprints/Items/LightningRuneItem.LightningRuneItem_C|GetEmmit _returnvalue_7) "None")))
    (:then_3
      (if (> _output_get 75.0)
        (bind _returnvalue_8 (Game|SpawnActorfromClass :Class "/Game/Blueprints/Items/EarthRuneItem.EarthRuneItem_C" :SpawnTransform (Math|Transform|MakeTransform (.location _returnvalue_4) (.rotation _returnvalue_4) "1,1,1") :CollisionHandlingOverride "Undefined" :Instigator 0))
        (Effects|SpawnEmitterAttached "/Game/Particles/P_UncommonMarker.P_UncommonMarker" (Variables|/Game/Blueprints/Items/EarthRuneItem.EarthRuneItem_C|GetEmmit _returnvalue_8) "None")))))

(fn SpawnPassive)

(fn SpawnActive
  (bind _defaultsceneroot (Variables|Default|GetDefaultSceneRoot))
  (bind _returnvalue (Transformation|GetWorldTransform _defaultsceneroot))
  (bind _returnvalue_2 (Transformation|GetWorldTransform _defaultsceneroot))
  (bind _returnvalue_3 (Transformation|GetWorldTransform _defaultsceneroot))
  (bind _output_get (Variables|Default|SetActiveChance (Math|Random|RandomFloatinRange 0.0 1e+02)))
  (Utilities|FlowControl|Sequence
    (:then_0
      (if (<= _output_get 33.0)
        (bind _returnvalue_4 (Game|SpawnActorfromClass :Class "/Game/Blueprints/Items/IcarusWingsItem.IcarusWingsItem_C" :SpawnTransform (Math|Transform|MakeTransform (.location _returnvalue) (.rotation _returnvalue) "1,1,1") :CollisionHandlingOverride "Undefined" :Instigator 0))
        (Effects|SpawnEmitterAttached "/Game/Particles/P_UncommonMarker.P_UncommonMarker" (Variables|/Game/Blueprints/Items/IcarusWingsItem.IcarusWingsItem_C|GetEmmit _returnvalue_4) "None")))
    (:then_1
      (if (and (> _output_get 33.0) (<= _output_get 66.0))
        (bind _returnvalue_5 (Game|SpawnActorfromClass :Class "/Game/Blueprints/Items/ZeusFuryItem.ZeusFuryItem_C" :SpawnTransform (Math|Transform|MakeTransform (.location _returnvalue_2) (.rotation _returnvalue_2) "1,1,1") :CollisionHandlingOverride "Undefined" :Instigator 0))
        (Effects|SpawnEmitterAttached "/Game/Particles/P_UncommonMarker.P_UncommonMarker" (Variables|/Game/Blueprints/Items/ZeusFuryItem.ZeusFuryItem_C|GetEmmit _returnvalue_5) "None")))
    (:then_2
      (if (> _output_get 66.0)
        (bind _returnvalue_6 (Game|SpawnActorfromClass :Class "/Game/Blueprints/Items/ActiveItem.ActiveItem_C" :SpawnTransform (Math|Transform|MakeTransform (.location _returnvalue_3) (.rotation _returnvalue_3) "1,1,1") :CollisionHandlingOverride "Undefined" :Instigator 0))
        (Effects|SpawnEmitterAttached "/Game/Particles/P_UncommonMarker.P_UncommonMarker" (Variables|/Game/Blueprints/Items/ActiveItem.ActiveItem_C|GetEmmit _returnvalue_6) "None")))))

(fn SpawnGoldStat
  (bind _defaultsceneroot (Variables|Default|GetDefaultSceneRoot))
  (bind _returnvalue (Transformation|GetWorldTransform _defaultsceneroot))
  (bind _returnvalue_2 (Transformation|GetWorldTransform _defaultsceneroot))
  (bind _returnvalue_3 (Transformation|GetWorldTransform _defaultsceneroot))
  (bind _output_get (Variables|Default|SetStatRuneChance (Math|Random|RandomFloatinRange 0.0 1e+02)))
  (Utilities|FlowControl|Sequence
    (:then_0
      (if (<= _output_get 33.0)
        (for _index (range 0 20)
          (Game|SpawnActorfromClass "/Game/Blueprints/Gold.Gold_C" (Math|Transform|MakeTransform (.location _returnvalue) (.rotation _returnvalue) "1,1,1") "Undefined" 0 0))
        (bind _returnvalue_4 (Game|SpawnActorfromClass :Class "/Game/Blueprints/Items/StatRuneItem.StatRuneItem_C" :SpawnTransform (Math|Transform|MakeTransform (.location _returnvalue) (.rotation _returnvalue) "1,1,1") :CollisionHandlingOverride "Undefined" :Instigator 0))
        (Effects|SpawnEmitterAttached "/Game/Particles/P_CommonMarker.P_CommonMarker" (Variables|/Game/Blueprints/Items/StatRuneItem.StatRuneItem_C|GetEmmit _returnvalue_4) "None")))
    (:then_1
      (if (and (> _output_get 33.0) (<= _output_get 66.0))
        (for _index_2 (range 0 20)
          (Game|SpawnActorfromClass "/Game/Blueprints/Gold.Gold_C" (Math|Transform|MakeTransform (.location _returnvalue_2) (.rotation _returnvalue_2) "1,1,1") "Undefined" 0 0))
        (bind _returnvalue_5 (Game|SpawnActorfromClass :Class "/Game/Blueprints/Items/StatRuneItem.StatRuneItem_C" :SpawnTransform (Math|Transform|MakeTransform (.location _returnvalue_2) (.rotation _returnvalue_2) "1,1,1") :CollisionHandlingOverride "Undefined" :Instigator 0))
        (Effects|SpawnEmitterAttached "/Game/Particles/P_CommonMarker.P_CommonMarker" (Variables|/Game/Blueprints/Items/StatRuneItem.StatRuneItem_C|GetEmmit _returnvalue_5) "None")))
    (:then_2
      (if (> _output_get 66.0)
        (for _index_3 (range 0 20)
          (Game|SpawnActorfromClass "/Game/Blueprints/Gold.Gold_C" (Math|Transform|MakeTransform (.location _returnvalue_3) (.rotation _returnvalue_3) "1,1,1") "Undefined" 0 0))
        (bind _returnvalue_6 (Game|SpawnActorfromClass :Class "/Game/Blueprints/Items/StatRuneItem.StatRuneItem_C" :SpawnTransform (Math|Transform|MakeTransform (.location _returnvalue_3) (.rotation _returnvalue_3) "1,1,1") :CollisionHandlingOverride "Undefined" :Instigator 0))
        (Effects|SpawnEmitterAttached "/Game/Particles/P_CommonMarker.P_CommonMarker" (Variables|/Game/Blueprints/Items/StatRuneItem.StatRuneItem_C|GetEmmit _returnvalue_6) "None")))))

(fn SpawnWeapon
  (bind _defaultsceneroot (Variables|Default|GetDefaultSceneRoot))
  (bind _returnvalue (Transformation|GetWorldTransform _defaultsceneroot))
  (bind _returnvalue_2 (Transformation|GetWorldTransform _defaultsceneroot))
  (bind _returnvalue_3 (Transformation|GetWorldTransform _defaultsceneroot))
  (bind _returnvalue_4 (Transformation|GetWorldTransform _defaultsceneroot))
  (bind _output_get (Variables|Default|SetRuneChance (Math|Random|RandomFloatinRange 0.0 1e+02)))
  (Utilities|FlowControl|Sequence
    (:then_0
      (if (<= _output_get 25.0)
        (bind _returnvalue_5 (Game|SpawnActorfromClass "/Game/Blueprints/Weapons/Xiphos.Xiphos_C" (Math|Transform|MakeTransform (.location _returnvalue) (.rotation _returnvalue) "1,1,1") "Undefined" 0 0))
        (Effects|SpawnEmitterAttached "/Game/Particles/P_UncommonMarker.P_UncommonMarker" (Variables|/Game/Blueprints/Weapons/Xiphos.Xiphos_C|GetEmmit _returnvalue_5) "None")))
    (:then_1
      (if (and (> _output_get 25.0) (<= _output_get 5e+01))
        (bind _returnvalue_6 (Game|SpawnActorfromClass "/Game/Blueprints/Weapons/Khopesh.Khopesh_C" (Math|Transform|MakeTransform (.location _returnvalue_2) (.rotation _returnvalue_2) "1,1,1") "Undefined" 0 0))
        (Effects|SpawnEmitterAttached "/Game/Particles/P_UncommonMarker.P_UncommonMarker" (Variables|/Game/Blueprints/Weapons/Khopesh.Khopesh_C|GetEmmit _returnvalue_6) "None")))
    (:then_2
      (if (and (> _output_get 5e+01) (<= _output_get 75.0))
        (bind _returnvalue_7 (Game|SpawnActorfromClass "/Game/Blueprints/Weapons/Dagger.Dagger_C" (Math|Transform|MakeTransform (.location _returnvalue_3) (.rotation _returnvalue_3) "1,1,1") "Undefined" 0 0))
        (Effects|SpawnEmitterAttached "/Game/Particles/P_UncommonMarker.P_UncommonMarker" (Variables|/Game/Blueprints/Weapons/Dagger.Dagger_C|GetEmmit _returnvalue_7) "None")))
    (:then_3
      (if (> _output_get 75.0)
        (bind _returnvalue_8 (Game|SpawnActorfromClass "/Game/Blueprints/Weapons/Axe.Axe_C" (Math|Transform|MakeTransform (.location _returnvalue_4) (.rotation _returnvalue_4) "1,1,1") "Undefined" 0 0))
        (Effects|SpawnEmitterAttached "/Game/Particles/P_UncommonMarker.P_UncommonMarker" (Variables|/Game/Blueprints/Weapons/Axe.Axe_C|GetEmmit _returnvalue_8) "None")))))