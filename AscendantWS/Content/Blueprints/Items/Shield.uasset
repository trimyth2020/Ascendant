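; Shield item actor that pulses area lightning damage around itself for a short time, sparing the first player's character.
; On BeginPlay it spawns a fire particle effect and starts a looping one-second timer.
; Each tick of that timer applies full radial damage at the actor's location and increments a counter, destroying the actor after the fifth strike.
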(event Custom|Strike
  (Game|Damage|ApplyRadialDamage 2e+01 (Transformation|GetActorLocation) 3e+02 "/Game/Blueprints/DamageTypes/LightningDamage.LightningDamage_C" (Utilities|Array|MakeArray (Game|GetPlayerCharacter 0)) self (Game|GetInstigatorController) true "ECC_Visibility")
  (bind _result (Math|Integer|IncrementInt (Variables|Default|GetLoops))
    (:%20%20
      (bind _output_get (Variables|Default|SetLoops _result))
      (if (>= _output_get 5)
        (Actor|DestroyActor)))))

(event EventBeginPlay
  (Effects|SpawnEmitterAttached "/Game/Particles/P_Fire.P_Fire" 0 "None" (Transformation|GetActorLocation))
  (Utilities|Time|SetTimerbyEvent (delegate Custom|Strike) 1.0 (<= (Variables|Default|GetLoops) 4)))

(fn ConstructionScript)