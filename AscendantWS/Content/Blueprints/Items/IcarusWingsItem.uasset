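; IcarusWingsItem is a pickup that puts the Icarus wings item into the player's inventory.
; InteractDetect acts only when its Target is the first player's character, cast to PlayerCharB.
; If the InventoryComponent holds fewer than three active items, it appends ItemStruc to ActiveItems and destroys itself; otherwise it stays in the world.
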(event EventInteractDetect
  (params (Target :type Object%20Object%20Reference))
  (bind _returnvalue (Game|GetPlayerCharacter 0))
  (if (== Target _returnvalue)
    (bind _asplayer_char_b (Utilities|Casting|CastToPlayerCharB _returnvalue))
    (if (< (Utilities|Array|Length (Variables|/Game/Blueprints/InventoryComponent.InventoryComponent_C|GetActiveItems (Variables|/Game/PlayerCharacter/PlayerCharB.PlayerCharB_C|GetInventoryComponent _asplayer_char_b))) 3)
      (Utilities|Array|Add (Variables|/Game/Blueprints/InventoryComponent.InventoryComponent_C|GetActiveItems (Variables|/Game/PlayerCharacter/PlayerCharB.PlayerCharB_C|GetInventoryComponent _asplayer_char_b)) (Variables|Default|GetItemStruc))
      (Actor|DestroyActor))))

(fn ConstructionScript)