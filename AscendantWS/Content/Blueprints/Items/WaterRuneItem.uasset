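; Water rune pickup item that adds itself to the player's inventory on contact.
; When the player character overlaps its sphere, it casts to PlayerCharB and checks that the inventory component's MiscItems array holds fewer than nine entries.
; If there is room, it appends its item struct and destroys itself; otherwise it stays in the world.
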(event OnComponentBeginOverlap(Sphere1)
  (params (OverlappedComponent :type Primitive%20Component%20Object%20Reference) (OtherActor :type Actor%20Object%20Reference) (OtherComp :type Primitive%20Component%20Object%20Reference) (OtherBodyIndex :type Integer) (bFromSweep :type Boolean) (SweepResult :type Hit%20Result%20Structure%20%28by%20ref%29))
  (bind _returnvalue (Game|GetPlayerCharacter 0))
  (if (== OtherActor _returnvalue)
    (bind _asplayer_char_b (Utilities|Casting|CastToPlayerCharB _returnvalue))
    (if (< (Utilities|Array|Length (Variables|/Game/Blueprints/InventoryComponent.InventoryComponent_C|GetMiscItems (Variables|/Game/PlayerCharacter/PlayerCharB.PlayerCharB_C|GetInventoryComponent _asplayer_char_b))) 9)
      (Utilities|Array|Add (Variables|/Game/Blueprints/InventoryComponent.InventoryComponent_C|GetMiscItems (Variables|/Game/PlayerCharacter/PlayerCharB.PlayerCharB_C|GetInventoryComponent _asplayer_char_b)) (Variables|Default|GetItemStruc))
      (Actor|DestroyActor))))

(fn ConstructionScript)