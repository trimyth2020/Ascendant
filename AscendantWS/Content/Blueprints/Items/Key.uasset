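; Key pickup actor that flies to the player and adds to their key count, despawning after a minute if left uncollected.
; Any overlap with KeyTrigger plays a timeline that lerps the key from its current location toward player character 0.
; On arrival within tolerance, it casts the overlapping actor to PlayerCharB, increments its InventoryComponent key count and destroys itself.
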(event OnComponentBeginOverlap(KeyTrigger)
  (params (OverlappedComponent :type Primitive%20Component%20Object%20Reference) (OtherActor :type Actor%20Object%20Reference) (OtherComp :type Primitive%20Component%20Object%20Reference) (OtherBodyIndex :type Integer) (bFromSweep :type Boolean) (SweepResult :type Hit%20Result%20Structure%20%28by%20ref%29))
  (bind _returnvalue (Transformation|GetActorLocation))
  (bind _returnvalue_2 (Game|GetPlayerCharacter 0))
  (bind _returnvalue_3 (Transformation|GetActorLocation _returnvalue_2))
  (bind _newtrack_0 (Timeline|Timeline_0 Play)
    (:Update
      (Transformation|SetActorLocation (Math|Vector|Lerp(Vector) _returnvalue _returnvalue_3 _newtrack_0) false false)
      (if (Class|KismetMathLibrary|NearlyEqualTransformTransform (Math|Conversions|ToTransform(Vector) _returnvalue) (Math|Conversions|ToTransform(Vector) _returnvalue_3) 1e+01 1e+01 1.0)
        (bind _asplayer_char_b (Utilities|Casting|CastToPlayerCharB OtherActor))
        (Math|Integer|IncrementInt (Variables|/Game/Blueprints/InventoryComponent.InventoryComponent_C|GetKeys (Variables|/Game/PlayerCharacter/PlayerCharB.PlayerCharB_C|GetInventoryComponent _asplayer_char_b))
          (:%20%20
            (Actor|DestroyActor)))))))

(event Custom|Despawn
  (Actor|DestroyActor))

(event EventBeginPlay
  (Utilities|Time|SetTimerbyEvent (delegate Custom|Despawn) 6e+01))

(fn ConstructionScript)