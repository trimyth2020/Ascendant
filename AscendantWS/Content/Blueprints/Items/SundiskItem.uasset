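; Sundisk item actor that creates a short-lived fire area effect, dealing radial fire damage around itself.
; On BeginPlay it spawns a fire circle emitter at the player's feet and starts a one-second repeating timer.
; Each tick damages actors around the item's own location, sparing the player, and increments a loop counter.
; When the counter reaches its limit, the emitter and actor are destroyed.
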(event Custom|CustomEvent_0
  (Game|Damage|ApplyRadialDamage 2e+01 (Transformation|GetActorLocation) 3e+02 "/Game/Blueprints/DamageTypes/FireDamage.FireDamage_C" (Utilities|Array|MakeArray (Game|GetPlayerCharacter 0)) self (Game|GetInstigatorController) true "ECC_Visibility")
  (Development|PrintString "Radial damage")
  (bind _result (Math|Integer|IncrementInt (Variables|Default|GetLoops))
    (:%20%20
      (bind _output_get (Variables|Default|SetLoops _result))
      (if (>= _output_get 5)
        (Components|DestroyComponent (stale EventBeginPlay _returnvalue_3))
        (Actor|DestroyActor)))))

(event EventBeginPlay
  (bind _returnvalue (Game|GetPlayerCharacter 0))
  (bind _returnvalue_2 (Transformation|GetActorTransform _returnvalue))
  (bind _returnvalue_3 (Effects|SpawnEmitteratLocation "/Game/Particles/P_FireCircle.P_FireCircle" (+ (.location _returnvalue_2) "0, 0,-90.000000") (.rotation _returnvalue_2)))
  (Utilities|Time|SetTimerbyEvent (delegate Custom|CustomEvent_0) 1.0 (<= (Variables|Default|GetLoops) 4)))

(fn ConstructionScript)