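; DropSpawner is a one-shot loot actor that spawns a random pickup drop on BeginPlay, then destroys itself.
; A single random roll picks one of four equally likely drops: a gold pile, a key, a stat rune with gold, or a health pile.
; Keys and stat runes get an attached marker emitter.
; Health pickups scatter with random XY offsets from the root's relative transform, while the others spawn at the actor's position.
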(event EventBeginPlay
  (bind _output_get (Variables|Default|SetDropChance (Math|Random|RandomFloatinRange 0.0 1e+02)))
  (Utilities|FlowControl|Sequence
    (:then_0
      (if (<= _output_get 25.0)
        (CallFunction|SpawnGold)
        (Actor|DestroyActor :!label _label)))
    (:then_1
      (if (and (> _output_get 25.0) (<= _output_get 5e+01))
        (CallFunction|SpawnKey)
        (goto _label)))
    (:then_2
      (if (and (> _output_get 5e+01) (<= _output_get 75.0))
        (CallFunction|SpawnStat)
        (goto _label)))
    (:then_3
      (if (> _output_get 75.0)
        (CallFunction|SpawnHealth)
        (goto _label)))))

(fn ConstructionScript)

(fn SpawnHealth
  (bind _defaultsceneroot (Variables|Default|GetDefaultSceneRoot))
  (bind _returnvalue (Transformation|GetRelativeTransform _defaultsceneroot))
  (for _index (range 0 19)
    (Game|SpawnActorfromClass "/Game/Blueprints/Health.Health_C" (Math|Transform|MakeTransform (Math|Vector|MakeVector (+ (.x (.location _returnvalue)) (Math|Random|RandomFloatinRange 0.0 3e+01)) (+ (.y (.location _returnvalue)) (Math|Random|RandomFloatinRange 0.0 3e+01)) (.z (.location _returnvalue))) (.rotation _returnvalue) "1,1,1") "Undefined" 0 0)))

(fn SpawnKey
  (bind _returnvalue (Transformation|GetActorTransform))
  (bind _returnvalue_2 (Game|SpawnActorfromClass "/Game/Blueprints/Items/Key.Key_C" (Math|Transform|MakeTransform (.location _returnvalue) (.rotation _returnvalue) "1,1,1") "Undefined" 0 0))
  (Effects|SpawnEmitterAttached "/Game/Particles/P_CommonMarker.P_CommonMarker" (Variables|/Game/Blueprints/Items/Key.Key_C|GetEmmit _returnvalue_2) "None"))

(fn SpawnGold
  (bind _returnvalue (Transformation|GetActorTransform))
  (for _index (range 0 19)
    (Game|SpawnActorfromClass "/Game/Blueprints/Gold.Gold_C" (Math|Transform|MakeTransform (.location _returnvalue) (.rotation _returnvalue) "1,1,1") "Undefined" 0 0)))

(fn SpawnStat
  (bind _defaultsceneroot (Variables|Default|GetDefaultSceneRoot))
  (bind _returnvalue (Transformation|GetWorldTransform _defaultsceneroot))
  (for _index (range 0 20)
    (Game|SpawnActorfromClass "/Game/Blueprints/Gold.Gold_C" (Math|Transform|MakeTransform (.location _returnvalue) (.rotation _returnvalue) "1,1,1") "Undefined" 0 0))
  (bind _returnvalue_2 (Game|SpawnActorfromClass :Class "/Game/Blueprints/Items/StatRuneItem.StatRuneItem_C" :SpawnTransform (Math|Transform|MakeTransform (.location _returnvalue) (.rotation _returnvalue) "1,1,1") :CollisionHandlingOverride "Undefined" :Instigator 0))
  (Effects|SpawnEmitterAttached "/Game/Particles/P_CommonMarker.P_CommonMarker" (Variables|/Game/Blueprints/Items/StatRuneItem.StatRuneItem_C|GetEmmit _returnvalue_2) "None"))