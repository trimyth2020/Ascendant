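; Health pickup actor that despawns 60 seconds after BeginPlay.
; When anything begins overlapping GoldTrigger and the player's PlayerStatsComponent Health is below MaxHealth, the ItemLerp timeline plays.
; Each update lerps the item from its current location toward the player, destroying it once the two locations nearly match.
; The Blueprint itself does not modify player health.
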(event OnComponentBeginOverlap(GoldTrigger)
  (params (OverlappedComponent :type Primitive%20Component%20Object%20Reference) (OtherActor :type Actor%20Object%20Reference) (OtherComp :type Primitive%20Component%20Object%20Reference) (OtherBodyIndex :type Integer) (bFromSweep :type Boolean) (SweepResult :type Hit%20Result%20Structure%20%28by%20ref%29))
  (bind _returnvalue (Transformation|GetActorLocation))
  (bind _returnvalue_2 (Game|GetPlayerCharacter 0))
  (bind _returnvalue_3 (Game|GetPlayerCharacter 0))
  (bind _returnvalue_4 (Transformation|GetActorLocation _returnvalue_2))
  (bind _asplayer_char_b (Utilities|Casting|CastToPlayerCharB _returnvalue_3))
  (bind _playerstatscomponent (Variables|/Game/PlayerCharacter/PlayerCharB.PlayerCharB_C|GetPlayerStatsComponent _asplayer_char_b))
  (if (< (Variables|/Game/Blueprints/PlayerStatsComponent.PlayerStatsComponent_C|GetHealth _playerstatscomponent) (Variables|/Game/Blueprints/PlayerStatsComponent.PlayerStatsComponent_C|GetMaxHealth _playerstatscomponent))
    (bind _newtrack_0 (Timeline|ItemLerp Play)
      (:Update
        (Transformation|SetActorLocation (Math|Vector|Lerp(Vector) _returnvalue _returnvalue_4 _newtrack_0) false false)
        (if (Class|KismetMathLibrary|NearlyEqualTransformTransform (Math|Conversions|ToTransform(Vector) _returnvalue) (Math|Conversions|ToTransform(Vector) _returnvalue_4) 3.0 3.0 3.0)
          (Actor|DestroyActor))))))

(event Custom|Despawn
  (Actor|DestroyActor))

(event EventBeginPlay
  (Utilities|Time|SetTimerbyEvent (delegate Custom|Despawn) 6e+01))

(fn ConstructionScript)