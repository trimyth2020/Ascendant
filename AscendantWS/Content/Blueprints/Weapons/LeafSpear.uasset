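; LeafSpear is a weapon pickup that adds its item struct to the player's inventory on interaction.
; BeginPlay randomizes one struct field from 0 to 3.
; InteractDetect appends it when fewer than two weapons are held, then destroys the actor.
; Otherwise it spawns the first weapon's class at the player's negated, scaled forward vector, without adding player location, and inserts itself at index 0 without removing that entry.
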(event EventBeginPlay
  (Variables|Default|SetItemStruc (Utilities|Struct|MakeWeaponItemStruc (.name (Variables|Default|GetItemStruc)) (.description (Variables|Default|GetItemStruc)) (.thumbnail (Variables|Default|GetItemStruc)) (.class (Variables|Default|GetItemStruc)) (.weaponmesh (Variables|Default|GetItemStruc)) (.weaponmaterial (Variables|Default|GetItemStruc)) (.weaponindex (Variables|Default|GetItemStruc)) (Math|Random|RandomIntegerinRange 0 3) (.equippeditems (Variables|Default|GetItemStruc)) (.attack (Variables|Default|GetItemStruc)) (.defense (Variables|Default|GetItemStruc)) (.attackspeed (Variables|Default|GetItemStruc)) (.damagetype (Variables|Default|GetItemStruc)))))

(event EventInteractDetect
  (params (Target :type Object%20Object%20Reference))
  (bind _returnvalue (Game|GetPlayerCharacter 0))
  (bind _itemstruc (Variables|Default|GetItemStruc))
  (bind _asplayer_char_b (Utilities|Casting|CastToPlayerCharB _returnvalue))
  (if (< (Utilities|Array|Length (Variables|/Game/Blueprints/InventoryComponent.InventoryComponent_C|GetWeaponItems (Variables|/Game/PlayerCharacter/PlayerCharB.PlayerCharB_C|GetInventoryComponent _asplayer_char_b))) 2)
    (Utilities|Array|Add (Variables|/Game/Blueprints/InventoryComponent.InventoryComponent_C|GetWeaponItems (Variables|/Game/PlayerCharacter/PlayerCharB.PlayerCharB_C|GetInventoryComponent _asplayer_char_b)) _itemstruc)
    (Actor|DestroyActor)
    (else
      (Game|SpawnActorfromClass (.class (Utilities|Array|Get(acopy) (Variables|/Game/Blueprints/InventoryComponent.InventoryComponent_C|GetWeaponItems (Variables|/Game/PlayerCharacter/PlayerCharB.PlayerCharB_C|GetInventoryComponent _asplayer_char_b)))) (Math|Conversions|ToTransform(Vector) (* (Transformation|GetActorForwardVector _returnvalue) -6e+02)) "Undefined" 0 0)
      (Utilities|Array|Insert (Variables|/Game/Blueprints/InventoryComponent.InventoryComponent_C|GetWeaponItems (Variables|/Game/PlayerCharacter/PlayerCharB.PlayerCharB_C|GetInventoryComponent _asplayer_char_b)) _itemstruc)
      (Actor|DestroyActor))))

(fn ConstructionScript)