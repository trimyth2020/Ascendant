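; Xiphos weapon pickup that adds its item struct to the player's inventory component when interacted with, then destroys itself.
; With fewer than two weapons held, InteractDetect appends the item.
; Otherwise it spawns the first slot's class at the player's forward vector times a negative offset, without adding player location.
; It then inserts the new item at index 0 without removing the old entry.
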(event EventInteractDetect
  (params (Target :type Object%20Object%20Reference))
  (bind _returnvalue (Game|GetPlayerCharacter 0))
  (bind _itemstruc (Variables|Default|GetItemStruc))
  (bind _asplayer_char_b (Utilities|Casting|CastToPlayerCharB _returnvalue))
  (if (< (Utilities|Array|Length (Variables|/Game/Blueprints/InventoryComponent.InventoryComponent_C|GetWeaponItems (Variables|/Game/PlayerCharacter/PlayerCharB.PlayerCharB_C|GetInventoryComponent _asplayer_char_b))) 2)
    (Utilities|Array|Add (Variables|/Game/Blueprints/InventoryComponent.InventoryComponent_C|GetWeaponItems (Variables|/Game/PlayerCharacter/PlayerCharB.PlayerCharB_C|GetInventoryComponent _asplayer_char_b)) _itemstruc)
    (Actor|DestroyActor)
    (else
      (Game|SpawnActorfromClass (.class (Utilities|Array|Get(acopy) (Variables|/Game/Blueprints/InventoryComponent.InventoryComponent_C|GetWeaponItems (Variables|/Game/PlayerCharacter/PlayerCharB.PlayerCharB_C|GetInventoryComponent _asplayer_char_b)))) (Math|Conversions|ToTransform(Vector) (* (Transformation|GetActorForwardVector _returnvalue) -6e+02)) "Undefined" 0 0)
      (Utilities|Array|Insert (Variables|/Game/Blueprints/InventoryComponent.InventoryComponent_C|GetWeaponItems (Variables|/Game/PlayerCharacter/PlayerCharB.PlayerCharB_C|GetInventoryComponent _asplayer_char_b)) _itemstruc)
      (Actor|DestroyActor))))

(fn ConstructionScript)