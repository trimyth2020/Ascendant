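; BindingPanel is a trap actor that temporarily roots PlayerCharB in place.
; When that character's capsule overlaps BindTrigger, it stops and disables the character's movement and turns off the trigger's collision.
; After a BindingTime delay, it restores walking mode and destroys itself, so each panel works only once.
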(event OnComponentBeginOverlap(BindTrigger)
  (params (OverlappedComponent :type Primitive%20Component%20Object%20Reference) (OtherActor :type Actor%20Object%20Reference) (OtherComp :type Primitive%20Component%20Object%20Reference) (OtherBodyIndex :type Integer) (bFromSweep :type Boolean) (SweepResult :type Hit%20Result%20Structure%20%28by%20ref%29))
  (bind _asplayer_char_b (Utilities|Casting|CastToPlayerCharB OtherActor))
  (if (== OtherComp (Variables|/Script/Engine.Character|GetCapsuleComponent _asplayer_char_b))
    (Components|Movement|StopMovementImmediately (Variables|/Script/Engine.Character|GetCharacterMovement _asplayer_char_b))
    (Pawn|Components|CharacterMovement|DisableMovement (Variables|/Script/Engine.Character|GetCharacterMovement _asplayer_char_b))
    (Collision|SetCollisionEnabled (Variables|Default|GetBindTrigger) "NoCollision")
    (Utilities|FlowControl|Delay (Variables|Default|GetBindingTime))
    (Pawn|Components|CharacterMovement|SetMovementMode (Variables|/Script/Engine.Character|GetCharacterMovement _asplayer_char_b) "MOVE_Walking" 0)
    (Actor|DestroyActor)))

(fn ConstructionScript)