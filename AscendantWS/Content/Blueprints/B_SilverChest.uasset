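; Silver chest that the player unlocks with a key to receive uncommon loot.
; InteractDetect checks the player inventory and deducts a key before a DoOnce gate, so repeat interactions still consume keys.
; The gate plays a timeline that moves and rotates the lid.
; When it finishes, a loop attaches uncommon-chest particles to the body, and a delayed DoN spawns one UncommonItemSpawner just above it.
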(event EventInteractDetect
  (params (Target :type Object%20Object%20Reference))
  (bind _returnvalue (Game|GetPlayerCharacter 0))
  (bind _silverchestbody (Variables|Default|GetSilverChestBody))
  (bind _returnvalue_2 (Transformation|GetWorldTransform _silverchestbody))
  (bind _asplayer_char_b (Utilities|Casting|CastToPlayerCharB _returnvalue))
  (if (>= (Variables|/Game/Blueprints/InventoryComponent.InventoryComponent_C|GetKeys (Variables|/Game/PlayerCharacter/PlayerCharB.PlayerCharB_C|GetInventoryComponent _asplayer_char_b)) 1)
    (bind _asplayer_char_b_2 (Utilities|Casting|CastToPlayerCharB _returnvalue))
    (bind _result (Math|Integer|DecrementInt (Variables|/Game/Blueprints/InventoryComponent.InventoryComponent_C|GetKeys (Variables|/Game/PlayerCharacter/PlayerCharB.PlayerCharB_C|GetInventoryComponent _asplayer_char_b_2)))
      (:%20%20
        (Variables|/Game/Blueprints/InventoryComponent.InventoryComponent_C|SetKeys (Variables|/Game/PlayerCharacter/PlayerCharB.PlayerCharB_C|GetInventoryComponent _asplayer_char_b_2) _result)
        (Utilities|FlowControl|DoOnce false
          (:Completed
            (bind (_direction _lidrotation _lidlocationx _lidlocationz) (Timeline|ChestOpen Play)
              (:Update
                (Transformation|SetRelativeTransform (Variables|Default|GetSilverChestLid) (Math|Transform|MakeTransform (Math|Vector|MakeVector (.x _lidlocationx) 0.0 (.z _lidlocationz)) (Math|Rotator|MakeRotator 0.0 (.y _lidrotation) 0.0) "1,1,1") false false))
              (:Finished
                (for _index (range 0 2)
                  (Effects|SpawnEmitterAttached "/Game/Particles/P_UncommonChest.P_UncommonChest" (Variables|Default|GetSilverChestBody) "None")
                  (Utilities|FlowControl|Delay 0.5)
                  (Utilities|FlowControl|DoN 1
                    (:Exit
                      (Game|SpawnActorfromClass "/Game/Blueprints/UncommonItemSpawner.UncommonItemSpawner_C" (Math|Transform|MakeTransform (+ (.location _returnvalue_2) "0, 0,40.000000") (.rotation _returnvalue_2) "1,1,1") "Undefined" 0 0))))))))))))

(fn ConstructionScript)