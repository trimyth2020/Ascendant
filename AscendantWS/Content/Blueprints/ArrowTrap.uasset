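; Arrow trap actor that fires projectiles when the player enters its trigger box.
; Box overlap fires only for PlayerCharB's capsule component, then calls Spawn three times at one-second intervals.
; Spawn creates a FirstPersonProjectile at the Scene component's world location and rotation, so that component sets the firing point and direction.
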(event OnComponentBeginOverlap(Box)
  (params (OverlappedComponent :type Primitive%20Component%20Object%20Reference) (OtherActor :type Actor%20Object%20Reference) (OtherComp :type Primitive%20Component%20Object%20Reference) (OtherBodyIndex :type Integer) (bFromSweep :type Boolean) (SweepResult :type Hit%20Result%20Structure%20%28by%20ref%29))
  (bind _asplayer_char_b (Utilities|Casting|CastToPlayerCharB OtherActor))
  (if (== OtherComp (Variables|/Script/Engine.Character|GetCapsuleComponent _asplayer_char_b))
    (CallFunction|Spawn)
    (Utilities|FlowControl|Delay 1.0)
    (CallFunction|Spawn)
    (Utilities|FlowControl|Delay 1.0)
    (CallFunction|Spawn)))

(fn ConstructionScript)

(fn Spawn
  (bind _scene (Variables|Default|GetScene))
  (bind _returnvalue (Transformation|GetWorldTransform _scene))
  (Game|SpawnActorfromClass "/Game/AI/RangedAI/FirstPersonBP/Blueprints/FirstPersonProjectile.FirstPersonProjectile_C" (Math|Transform|MakeTransform (.location _returnvalue) (.rotation _returnvalue) "1,1,1") "Undefined" 0 0))