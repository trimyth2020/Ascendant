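; MediumStrucSpawner is a spawner that places a random medium plot structure at its own transform.
; SpawnMediumStructure rolls a float from 0 to 100 and spawns MediumPlot1_BP or MediumPlot2_BP at roughly even odds, with a narrow gap just above 50 that spawns nothing.
; Both the Construction Script and BeginPlay call this function, each with an independent roll and no check for an existing structure.
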(event EventBeginPlay
  (CallFunction|SpawnMediumStructure))

(event Collision|EventActorBeginOverlap
  (params (OtherActor :type Actor%20Object%20Reference)))

(event EventTick
  (params (DeltaSeconds :type Float%20%28single-precision%29)))

(fn ConstructionScript
  (CallFunction|SpawnMediumStructure))

(fn SpawnMediumStructure
  (bind _returnvalue (Transformation|GetActorTransform))
  (bind _output_get (Variables|Default|SetRandomValue (Math|Random|RandomFloatinRange 0.0 1e+02)))
  (if (Math|Float|InRange(Float) _output_get 0.0 5e+01)
    (Game|SpawnActorfromClass "/Game/Blueprints/StructureBPs/MediumPlot1_BP.MediumPlot1_BP_C" _returnvalue "Undefined" 0 0)
    (elif (Math|Float|InRange(Float) _output_get 50.099998 1e+02)
      (Game|SpawnActorfromClass "/Game/Blueprints/StructureBPs/MediumPlot2_BP.MediumPlot2_BP_C" _returnvalue "Undefined" 0 0))))