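; Item spawner actor that places one random elemental rune pickup (Fire, Water, Lightning or Earth) when play begins.
; BeginPlay calls SpawnItem, which rolls a random float and uses four exclusive range checks to give each rune type an equal chance.
; The chosen rune spawns at the spawner root's location and rotation and is returned, though BeginPlay does not use the result.
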(event EventBeginPlay
  (CallFunction|SpawnItem))

(fn ConstructionScript)

(fn SpawnItem
  (bind _defaultsceneroot (Variables|Default|GetDefaultSceneRoot))
  (bind _returnvalue (Transformation|GetWorldTransform _defaultsceneroot))
  (bind _returnvalue_2 (Transformation|GetWorldTransform _defaultsceneroot))
  (bind _returnvalue_3 (Transformation|GetWorldTransform _defaultsceneroot))
  (bind _returnvalue_4 (Transformation|GetWorldTransform _defaultsceneroot))
  (bind _output_get (Variables|Default|SetItemChance (Math|Random|RandomFloatinRange 0.0 1e+02)))
  (Utilities|FlowControl|Sequence
    (:then_0
      (if (<= _output_get 25.0)
        (bind _returnvalue_5 (Game|SpawnActorfromClass :Class "/Game/Blueprints/Items/FireRuneItem.FireRuneItem_C" :SpawnTransform (Math|Transform|MakeTransform (.location _returnvalue) (.rotation _returnvalue) "1,1,1") :CollisionHandlingOverride "Undefined" :Instigator 0))
        (return _returnvalue_5)))
    (:then_1
      (if (and (> _output_get 25.0) (<= _output_get 5e+01))
        (bind _returnvalue_6 (Game|SpawnActorfromClass :Class "/Game/Blueprints/Items/WaterRuneItem.WaterRuneItem_C" :SpawnTransform (Math|Transform|MakeTransform (.location _returnvalue_2) (.rotation _returnvalue_2) "1,1,1") :CollisionHandlingOverride "Undefined" :Instigator 0))
        (return _returnvalue_6)))
    (:then_2
      (if (and (> _output_get 5e+01) (<= _output_get 75.0))
        (bind _returnvalue_7 (Game|SpawnActorfromClass :Class "/Game/Blueprints/Items/LightningRuneItem.LightningRuneItem_C" :SpawnTransform (Math|Transform|MakeTransform (.location _returnvalue_3) (.rotation _returnvalue_3) "1,1,1") :CollisionHandlingOverride "Undefined" :Instigator 0))
        (return _returnvalue_7)))
    (:then_3
      (if (> _output_get 75.0)
        (bind _returnvalue_8 (Game|SpawnActorfromClass :Class "/Game/Blueprints/Items/EarthRuneItem.EarthRuneItem_C" :SpawnTransform (Math|Transform|MakeTransform (.location _returnvalue_4) (.rotation _returnvalue_4) "1,1,1") :CollisionHandlingOverride "Undefined" :Instigator 0))
        (return _returnvalue_8)))))