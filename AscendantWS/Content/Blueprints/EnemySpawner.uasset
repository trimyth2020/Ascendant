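; Enemy spawner that randomly places up to three AI enemies around its SpawnPoint when play begins.
; A three-pin Sequence repeats one roll: above EnemySpawnChance spawns an enemy, so higher values mean fewer spawns.
; A second roll picks NPC at or above MeleeChance, otherwise Ranged_AI, each with its behavior tree.
; Random positive X/Y offsets place ranged enemies farther out than NPCs.
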(event EventBeginPlay
  (CallFunction|EnemySpawn))

(fn ConstructionScript)

(fn EnemySpawn
  (bind _spawnpoint (Variables|Default|GetSpawnPoint))
  (bind _spawnpoint_2 (Variables|Default|GetSpawnPoint))
  (bind _returnvalue (Transformation|GetWorldLocation _spawnpoint))
  (bind _returnvalue_2 (Transformation|GetWorldLocation _spawnpoint_2))
  (Utilities|FlowControl|Sequence
    (:then_0
      _)
    (:then_1
      _)
    (:then_2
      _))
  ;[1 1 1] Chance of a chest spawning
  (if (> (Math|Random|RandomFloatinRange 0.0 1e+02) (Variables|Default|GetEnemySpawnChance))
    ;[1 1 1] Chance of being a small chest
    (if (>= (Math|Random|RandomFloatinRange 0.0 1e+02) (Variables|Default|GetMeleeChance))
      (AI|SpawnAIFromClass "/Game/AI/NPC/NPC.NPC_C" "/Game/AI/NPC/NPC_BT.NPC_BT" (Math|Vector|MakeVector (+ (.x _returnvalue_2) (Math|Random|RandomFloatinRange 2e+01 5e+01)) (+ (.y _returnvalue_2) (Math|Random|RandomFloatinRange 2e+01 5e+01)) (.z _returnvalue_2)) "0, 0, 0" false)
      (else
        (AI|SpawnAIFromClass "/Game/AI/RangedAI/Ranged_AI.Ranged_AI_C" "/Game/AI/RangedAI/Ranged_BT.Ranged_BT" (Math|Vector|MakeVector (+ (.x _returnvalue) (Math|Random|RandomFloatinRange 5e+01 8e+01)) (+ (.y _returnvalue) (Math|Random|RandomFloatinRange 5e+01 8e+01)) (.z _returnvalue)) "0, 0, 0" false)))))