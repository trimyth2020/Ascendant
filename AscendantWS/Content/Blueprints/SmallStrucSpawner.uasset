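; Spawner actor that places one of three small plot Blueprints, picked at random, at its own transform.
; SpawnSmallStructure rolls a random float and compares it against three roughly equal ranges to choose SmallPlot1_BP, SmallPlot2_BP or SmallPlot3_BP.
; Both the Construction Script and BeginPlay call this function, each making its own roll and spawn attempt, with no tracking or cleanup of earlier spawns.
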(event EventBeginPlay
  (CallFunction|SpawnSmallStructure))

(event Collision|EventActorBeginOverlap
  (params (OtherActor :type Actor%20Object%20Reference)))

(event EventTick
  (params (DeltaSeconds :type Float%20%28single-precision%29)))

(fn ConstructionScript
  (CallFunction|SpawnSmallStructure))

(fn SpawnSmallStructure
  (bind _returnvalue (Transformation|GetActorTransform))
  (bind _output_get (Variables|Default|SetRandomValue (Math|Random|RandomFloatinRange 0.0 1e+02)))
  (if (Math|Float|InRange(Float) _output_get 0.0 33.0)
    (Game|SpawnActorfromClass "/Game/Blueprints/StructureBPs/SmallPlot1_BP.SmallPlot1_BP_C" _returnvalue "Undefined" 0 0)
    (elif (Math|Float|InRange(Float) _output_get 33.0 66.0)
      (Game|SpawnActorfromClass "/Game/Blueprints/StructureBPs/SmallPlot2_BP.SmallPlot2_BP_C" _returnvalue "Undefined" 0 0)
      (elif (Math|Float|InRange(Float) _output_get 66.0 1e+02)
        (Game|SpawnActorfromClass "/Game/Blueprints/StructureBPs/SmallPlot3_BP.SmallPlot3_BP_C" _returnvalue "Undefined" 0 0)))))