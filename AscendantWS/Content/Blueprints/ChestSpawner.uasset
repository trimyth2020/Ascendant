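; Chest spawner actor that randomly places a treasure chest at its SpawnPoint on BeginPlay.
; ChestSpawn spawns only when a percentage roll exceeds ChestSpawnChance, so higher values mean fewer chests.
; A second roll against SmallChance picks small or big, then a weighted roll picks bronze, silver or gold, with gold rarest.
; Successful spawns print a debug string, which includes the actor name for small chests.
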(event EventBeginPlay
  (CallFunction|ChestSpawn))

(fn ConstructionScript)

(fn ChestSpawn
  (bind _spawnpoint (Variables|Default|GetSpawnPoint))
  (bind _spawnpoint_2 (Variables|Default|GetSpawnPoint))
  (bind _returnvalue (Transformation|GetWorldTransform _spawnpoint))
  (bind _returnvalue_2 (Transformation|GetWorldTransform _spawnpoint))
  (bind _returnvalue_3 (Transformation|GetWorldTransform _spawnpoint))
  (bind _returnvalue_4 (Transformation|GetWorldTransform _spawnpoint_2))
  (bind _returnvalue_5 (Transformation|GetWorldTransform _spawnpoint_2))
  (bind _returnvalue_6 (Transformation|GetWorldTransform _spawnpoint_2))
  ;[1 1 1] Chance of a chest spawning
  (if (> (Math|Random|RandomFloatinRange 0.0 1e+02) (Variables|Default|GetChestSpawnChance))
    ;[1 1 1] Chance of being a small chest
    (if (>= (Math|Random|RandomFloatinRange 0.0 1e+02) (Variables|Default|GetSmallChance))
      ;[1 1 1] Calculates the rarity of the big chest
      (bind _output_get (Variables|Default|SetBigRandom (Math|Random|RandomFloatinRange 0.0 1e+02)))
      (Utilities|FlowControl|Sequence
        (:then_0
          (if (<= _output_get 4e+01)
            ;[1 1 1] Spawns a big chest
            (Game|SpawnActorfromClass "/Game/Blueprints/BigBronzeChest.BigBronzeChest_C" (Math|Transform|MakeTransform (.location _returnvalue_2) (.rotation _returnvalue_2) "1,1,1") "Undefined" 0 0)
            (Development|PrintString "Spawned" :!label _label)))
        (:then_1
          (if (and (> _output_get 4e+01) (<= _output_get 9e+01))
            (Game|SpawnActorfromClass "/Game/Blueprints/BigSilverChest.BigSilverChest_C" (Math|Transform|MakeTransform (.location _returnvalue_3) (.rotation _returnvalue_3) "1,1,1") "Undefined" 0 0)
            (goto _label)))
        (:then_2
          (if (> _output_get 9e+01)
            (Game|SpawnActorfromClass "/Game/Blueprints/BigGoldChest.BigGoldChest_C" (Math|Transform|MakeTransform (.location _returnvalue) (.rotation _returnvalue) "1,1,1") "Undefined" 0 0)
            (goto _label))))
      (else
        ;[1 1 1] Calculates the rarity of the small chest
        (bind _output_get_2 (Variables|Default|SetSmallRandom (Math|Random|RandomFloatinRange 0.0 1e+02)))
        (Utilities|FlowControl|Sequence
          (:then_0
            (if (<= _output_get_2 4e+01)
              ;[1 1 1] Spawns a small chest
              (bind _returnvalue_7 (Game|SpawnActorfromClass "/Game/Blueprints/BronzeChest.BronzeChest_C" (Math|Transform|MakeTransform (.location _returnvalue_4) (.rotation _returnvalue_4) "1,1,1") "Undefined" 0 0))
              (Variables|Default|SetSpawnedActor _returnvalue_7)
              (Development|PrintString (Utilities|String|Append "Spawned: " (Utilities|GetDisplayName (Variables|Default|GetSpawnedActor))) :!label _label_2)))
          (:then_1
            (if (and (> _output_get_2 4e+01) (<= _output_get_2 9e+01))
              (bind _returnvalue_8 (Game|SpawnActorfromClass "/Game/Blueprints/SilverChest.SilverChest_C" (Math|Transform|MakeTransform (.location _returnvalue_5) (.rotation _returnvalue_5) "1,1,1") "Undefined" 0 0))
              (Variables|Default|SetSpawnedActor _returnvalue_8)
              (goto _label_2)))
          (:then_2
            (if (> _output_get_2 9e+01)
              (bind _returnvalue_9 (Game|SpawnActorfromClass "/Game/Blueprints/GoldChest.GoldChest_C" (Math|Transform|MakeTransform (.location _returnvalue_6) (.rotation _returnvalue_6) "1,1,1") "Undefined" 0 0))
              (Variables|Default|SetSpawnedActor _returnvalue_9)
              (goto _label_2))))))))